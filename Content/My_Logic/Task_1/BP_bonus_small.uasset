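; BP_bonus_small is a moving bonus pickup that sends a shrink-ball effect when it touches the platform.
; Each tick it moves with a swept world offset along its direction and speed.
; Overlapping BP_Platform sends a half-size ScaleBallFunc message to every actor implementing My_Interface, then destroys the pickup.
; Overlapping a KillZVolume destroys it with no effect.
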(event EventBeginPlay)

(event Collision|EventActorBeginOverlap
  (params (OtherActor :type Actor%20Object%20Reference))
  (Utilities|FlowControl|Sequence
    (:then_0
      (Utilities|Casting|CastToKillZVolume OtherActor)
      (Actor|DestroyActor))
    (:then_1
      (Utilities|Casting|CastToBP_Platform OtherActor)
      (bind _outactors (Actor|GetAllActorswithInterface "/Game/My_Logic/Task_1/My_Interface.My_Interface_C"))
      (Class|MyInterface|ScaleBallFunc(Message) _outactors "0.500000,0.500000,0.500000")
      (Actor|DestroyActor))))

(event EventTick
  (params (DeltaSeconds :type Float%20%28single-precision%29))
  (Transformation|AddActorWorldOffset (* (* (Variables|Default|GetDerection) (Variables|Default|GetSpeed)) DeltaSeconds) true))

(fn ConstructionScript)