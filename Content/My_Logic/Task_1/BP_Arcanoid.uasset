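; BP_Arcanoid is an Arkanoid-style brick field that breaks apart when hit and can drop bonuses.
; The construction script builds an X-by-Y grid of static mesh components with configurable spacing.
; Each hit destroys the struck component, increments and prints Score, then randomly spawns a big bonus, or failing that possibly a small one, at the hit location.
; A My_Interface score broadcast exists but is not wired to run.
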(event EventBeginPlay)

(event Collision|EventActorBeginOverlap
  (params (OtherActor :type Actor%20Object%20Reference)))

(event EventTick
  (params (DeltaSeconds :type Float%20%28single-precision%29)))

(event Collision|EventHit
  (params (MyComp :type Primitive%20Component%20Object%20Reference) (Other :type Actor%20Object%20Reference) (OtherComp :type Primitive%20Component%20Object%20Reference) (bSelfMoved :type Boolean) (HitLocation :type Vector :default "0, 0, 0") (HitNormal :type Vector :default "0, 0, 0") (NormalImpulse :type Vector :default "0, 0, 0") (Hit :type Hit%20Result%20Structure%20%28by%20ref%29))
  (Utilities|FlowControl|Sequence
    (:then_0
      (Components|DestroyComponent MyComp)
      (bind _result (Math|Integer|IncrementInt (Variables|Default|GetScore))
        (:%20%20
          (Development|PrintString (Utilities|String|ToString(Integer) _result))
          (Development|PrintString "Score: "))))
    (:then_1
      (if (> (Math|Random|RandomFloatinRange 0.0 1.2) 1.0)
        (Game|SpawnActorfromClass "/Game/My_Logic/Task_1/BP_bonus_big.BP_bonus_big_C" (Math|Transform|MakeTransform HitLocation) "Undefined" 0 0)
        (elif (> (Math|Random|RandomFloatinRange 0.0 1.2) 1.0)
          (Game|SpawnActorfromClass "/Game/My_Logic/Task_1/BP_bonus_small.BP_bonus_small_C" (Math|Transform|MakeTransform HitLocation) "Undefined" 0 0))))))

(fn ConstructionScript
  (for _index (range 0 (- (Variables|Default|GetX) 1))
    (for _index_2 (range 0 (- (Variables|Default|GetY) 1))
      (AddComponent|AddStaticMeshComponent false (Math|Transform|MakeTransform (Math|Vector|MakeVector (Math|Conversions|ToFloat(Integer) (* _index (Variables|Default|GetX_dist))) (Math|Conversions|ToFloat(Integer) (* _index_2 (Variables|Default|GetY_dist))) 0.0))))))