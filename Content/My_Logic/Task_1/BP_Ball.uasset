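; BP_Ball is a bouncing ball actor for a paddle-style game with BP_Platform.
; Tick moves it along its direction and speed with a swept offset, reflecting the direction off the surface normal on blocking hits.
; Overlapping a KillZVolume subtracts a life from every BP_Platform and destroys the ball.
; ScaleBallFunc applies a temporary scale, then restores normal size after a delay.
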(event EventBeginPlay)

(event Collision|EventActorBeginOverlap
  (params (OtherActor :type Actor%20Object%20Reference))
  (Utilities|Casting|CastToKillZVolume OtherActor)
  (bind _outactors (Actor|GetAllActorsOfClass "/Game/My_Logic/Task_1/BP_Platform.BP_Platform_C"))
  (Default|SubstructLife _outactors)
  (Actor|DestroyActor))

(event EventTick
  (params (DeltaSeconds :type Float%20%28single-precision%29))
  (bind _sweephitresult (Transformation|AddActorWorldOffset (* (* (Variables|Default|GetDerection) (Variables|Default|GetSpeed)) DeltaSeconds) true))
  (if (.bBlockingHit (Collision|BreakHitResult _sweephitresult))
    (Variables|Default|SetDerection (Math|Vector|GetReflectionVector (Variables|Default|GetDerection) (.Normal (Collision|BreakHitResult _sweephitresult))))))

(event EventScaleBallFunc
  (params (Scale_ball :type Vector :default "0, 0, 0"))
  (Transformation|SetActorRelativeScale3D Scale_ball)
  (Utilities|FlowControl|Delay 5.0)
  (Transformation|SetActorRelativeScale3D "1.000000,1.000000,1.000000"))

(fn ConstructionScript)